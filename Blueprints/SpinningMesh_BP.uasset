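; SpinningMesh_BP is a spinning mesh actor with a configurable mesh and material that reacts to being hit by Ball_BP.
; The construction script applies StaticMeshToApply and MaterialToApply to the StaticMesh component.
; Tick adds RotationSpeed as local yaw each frame, without delta-time scaling.
; A hit from Ball_BP switches the first material slot to a dynamic instance of M_KillVolume.
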(event `self.ReceiveTick`
  (params (DeltaSeconds :type "Float (single-precision)"))
  (`SceneComponent.K2_AddLocalRotation` (`self.StaticMesh`) (`KismetMathLibrary.MakeRotator` 0.0 0.0 (`self.Rotation Speed`)) false false))

(event `self.ReceiveHit`
  (params (MyComp :type "PrimitiveComponent Object Reference") (Other :type "Actor Object Reference") (OtherComp :type "PrimitiveComponent Object Reference") (bSelfMoved :type Boolean) (HitLocation :type "Vector Structure") (HitNormal :type "Vector Structure") (NormalImpulse :type "Vector Structure") (Hit :type "HitResult Structure (by ref)"))
  (if (== Other "/Game/Ball/Ball_BP.Ball_BP")
    (`PrimitiveComponent.CreateDynamicMaterialInstance` (`self.StaticMesh`) 0 "/Game/Materials/M_KillVolume.M_KillVolume" "None")))

(fn `UserConstructionScript`
  (`StaticMeshComponent.SetStaticMesh` (`self.StaticMesh`) (`self.Static Mesh To Apply`))
  (`PrimitiveComponent.SetMaterial` (`self.StaticMesh`) 0 (`self.Material To Apply`)))