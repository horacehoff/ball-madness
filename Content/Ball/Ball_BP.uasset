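; Player ball for a timed level game, rolled with physics torque from input axes, with pause menu and gamepad rumble on fast hits.
; BeginPlay runs a hardware benchmark, creates the HUD, briefly locks input, and sets the countdown and Discord status by map name.
; Excessive speed triggers a limited respawn at the saved location, falling back to PlayerStart before game over.
; Tick drives the countdown through a one-second Delay, opening GameOverMap at zero.
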(event `InputAxis|LookUp`
  (params (AxisValue :type "Float (single-precision)"))
  ;[1 0 0.08349] Roll left/right
  (`PrimitiveComponent.AddTorqueInRadians` (`self.Ball`) (`KismetMathLibrary.MakeVector` (* (`self.RollTorque`) AxisValue -1.0)) "None" false))

(event `InputAxis|Turn`
  (params (AxisValue :type "Float (single-precision)"))
  ;[1 0 0.01201] Roll forwards/backwards
  (`PrimitiveComponent.AddTorqueInRadians` (`self.Ball`) (`KismetMathLibrary.MakeVector` 0.0 (* (`self.RollTorque`) AxisValue)) "None" false))

(event `self.ReceiveTick`
  (params (DeltaSeconds :type "Float (single-precision)"))
  (if (> (`KismetMathLibrary.VSize` (`self.GetVelocity`)) 2500.0)
    (`self.Respawn`))
  (`self.Timer`))

(event `InputAction|Escape`
  (params (Key :type "Key Structure"))
  (:`Pressed`
    (bind _returnvalue (`|CreateWidget` "/Game/UI/Pause_HUD.Pause_HUD_C"))
    (bind _output_get (set `self.Pause_HUD` _returnvalue))
    (`UserWidget.AddToViewport` _output_get 0)
    (set `PlayerController.bShowMouseCursor` true (`GameplayStatics.GetPlayerController` 0))))

(event `self.ReceiveHit`
  (params (MyComp :type "PrimitiveComponent Object Reference") (Other :type "Actor Object Reference") (OtherComp :type "PrimitiveComponent Object Reference") (bSelfMoved :type Boolean) (HitLocation :type "Vector Structure") (HitNormal :type "Vector Structure") (NormalImpulse :type "Vector Structure") (Hit :type "HitResult Structure (by ref)"))
  (bind _forcefeedback (`self.ForceFeedback`))
  ;[0 0.06478 1] Vibrates the GamePad if activated
  (if (<= (`KismetMathLibrary.VSize` (`self.GetVelocity`)) 500.0)
    (`ForceFeedbackComponent.Stop` _forcefeedback)
    (else
      (`ForceFeedbackComponent.Play` (`self.ForceFeedback`) 0.0)
      (`KismetSystemLibrary.Delay` 0.120355)
      (`ForceFeedbackComponent.Stop` _forcefeedback))))

(event `self.ReceiveBeginPlay`
  (bind _returnvalue (`GameUserSettings.GetGameUserSettings`))
  (`GameUserSettings.RunHardwareBenchmark` _returnvalue 10 1.0 1.0)
  (`GameUserSettings.SetFrameRateLimit` _returnvalue 0.0)
  (`GameUserSettings.ApplySettings` _returnvalue true)
  (`GameUserSettings.ApplyHardwareBenchmarkResults` _returnvalue)
  (bind _outactors (`GameplayStatics.GetAllActorsOfClass` "/Script/Engine.PlayerStart"))
  (bind _output_get (set `self.LastSavedLocation` (`self.K2_GetActorLocation` (`|GetArrayItem` _outactors))))
  (set `self.DefaultLocation` _output_get)
  (set `self.RespawnCounter` 0)
  (`self.SetTimerByMap`)
  (set `self.HasGameStarted` false)
  (bind _returnvalue_2 (`|CreateWidget` "/Game/UI/PlayerData_HUD.PlayerData_HUD_C"))
  (`UserWidget.AddToViewport` _returnvalue_2 0)
  (`self.DisableInput` (`GameplayStatics.GetPlayerController` 0))
  (`KismetSystemLibrary.Delay` 2.25)
  (`self.EnableInput` (`GameplayStatics.GetPlayerController` 0))
  (`self.SetDiscordStatusByMap`)
  (bind _returnvalue_3 (`GameplayStatics.GetCurrentLevelName` true))
  (if (`KismetStringLibrary.NotEqual_StrStr` _returnvalue_3 "MainMap")
    (set `self.HasGameStarted` true)
    (else
      (set `self.HasGameStarted` false)))
  (`KismetSystemLibrary.ExecuteConsoleCommand` "DisableAllScreenMessages" null))

(fn `Respawn`
  (if (< (`self.RespawnCounter`) 3)
    (set `self.RespawnCounter` (+ (`self.RespawnCounter`) 1))
    (`self.K2_SetActorLocation` (`self.LastSavedLocation`) false true)
    (`PrimitiveComponent.SetAllPhysicsLinearVelocity` (`self.Ball`) (0.0 0.0 0.0) false)
    (`PrimitiveComponent.SetPhysicsAngularVelocityInRadians` (`self.Ball`) (0.0 0.0 0.0) false "None")
    (`GameplayStatics.PlaySound2D` "/Game/Retro_8Bit_Sounds/Teleport/Cues/retro_teleport_warp_effect_15_Cue.retro_teleport_warp_effect_15_Cue" 1.5 1.0 0.0 null null)
    (elif (not (== (`self.DefaultLocation`) (`self.LastSavedLocation`) :`ErrorTolerance` 0.01))
      (set `self.RespawnCounter` 0)
      (bind _output_get (set `self.LastSavedLocation` (`self.DefaultLocation`)))
      (`self.K2_SetActorLocation` _output_get false true)
      (`PrimitiveComponent.SetAllPhysicsLinearVelocity` (`self.Ball`) (0.0 0.0 0.0) false)
      (`PrimitiveComponent.SetPhysicsAngularVelocityInRadians` (`self.Ball`) (0.0 0.0 0.0) false "None")
      (`GameplayStatics.PlaySound2D` "/Game/Retro_8Bit_Sounds/Teleport/Cues/retro_teleport_warp_effect_15_Cue.retro_teleport_warp_effect_15_Cue" 1.5 1.0 0.0 null null)
      (else
        (`GameplayStatics.OpenLevel` "GameOverMap")))))

(fn `SetDiscordStatus`
  (params (`Large key` :type String) (State :type String) (Details :type String)))

(fn `SetDiscordStatusByMap`
  (bind _returnvalue (`GameplayStatics.GetCurrentLevelName` true))
  (for _array_element (`KismetStringLibrary.GetCharacterArrayFromString` _returnvalue)
    (if (`KismetStringLibrary.IsNumeric` _array_element)
      (if (`KismetStringLibrary.EqualEqual_StrStr` _array_element "1")
        (`self.SetDiscordStatus` "largekey" "Playing...->1st map" "~~~~~~~~~~~~")
        (elif (`KismetStringLibrary.EqualEqual_StrStr` _array_element "2")
          (`self.SetDiscordStatus` "largekey" "Playing...->2nd map" "~~~~~~~~~~~~")
          (elif (`KismetStringLibrary.EqualEqual_StrStr` _array_element "3")
            (`self.SetDiscordStatus` "largekey" "Playing...->3rd map" "~~~~~~~~~~~~")
            (else
              (`self.SetDiscordStatus` "largekey" (`KismetStringLibrary.Concat_StrStr` "Playing...->" _array_element "th map") "~~~~~~~~~~~~"))))))))

(fn `SetRemainingTime`
  (params (Minutes :type Integer) (Seconds :type Integer))
  (set `self.Seconds` Seconds)
  (set `self.Minutes` Minutes))

(fn `SetTimerByMap`
  (bind _returnvalue (`GameplayStatics.GetCurrentLevelName` true))
  (if (`KismetStringLibrary.EqualEqual_StrStr` _returnvalue "MainMap")
    _
    (elif (`KismetStringLibrary.EqualEqual_StrStr` _returnvalue "MainMap1")
      (`self.SetRemainingTime` 1)
      (elif (`KismetStringLibrary.EqualEqual_StrStr` _returnvalue "MainMap2")
        (`self.SetRemainingTime` 0 15)
        (elif (`KismetStringLibrary.EqualEqual_StrStr` _returnvalue "MainMap3")
          (`self.SetRemainingTime` 0 14)
          (elif (`KismetStringLibrary.EqualEqual_StrStr` _returnvalue "MainMap4")
            (`self.SetRemainingTime` 0 19)
            (elif (`KismetStringLibrary.EqualEqual_StrStr` _returnvalue "MainMap5")
              (`self.SetRemainingTime` 0 25)
              (elif (`KismetStringLibrary.EqualEqual_StrStr` _returnvalue "MainMap6")
                (`self.SetRemainingTime` 0 25)
                (elif (`KismetStringLibrary.EqualEqual_StrStr` _returnvalue "MainMap7")
                  (`self.SetRemainingTime` 0 32)
                  (elif (`KismetStringLibrary.EqualEqual_StrStr` _returnvalue "MainMap8")
                    (`self.SetRemainingTime` 1 35)
                    (elif (`KismetStringLibrary.EqualEqual_StrStr` _returnvalue "Prototyping")
                      (`self.SetRemainingTime` 60)
                      (elif (`KismetStringLibrary.EqualEqual_StrStr` _returnvalue "BadMap")
                        (`self.SetRemainingTime` 3600)
                        (elif (`KismetStringLibrary.EqualEqual_StrStr` _returnvalue "BadMap1")
                          (`self.SetRemainingTime` 0 40)
                          (elif (`KismetStringLibrary.EqualEqual_StrStr` _returnvalue "BadMap2")
                            (`self.SetRemainingTime` 0 5000)
                            (elif (`KismetStringLibrary.EqualEqual_StrStr` _returnvalue "TrainingLevel1")
                              (`self.SetRemainingTime` 0 5000))))))))))))))))

(fn `UserConstructionScript`)