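; Kill volume actor that sends the game to GameOverMap when anything triggers an overlap on its Box component, with no check on the overlapping actor.
; On BeginPlay it creates a dynamic material instance from M_KillVolume on the Cube component.
; Tick runs through a one-second Delay into a FlipFlop that alternates the material's "Second Base Color" between orange-red and red as a pulsing warning.
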(event `self.ReceiveBeginPlay`
  (bind _returnvalue (`PrimitiveComponent.CreateDynamicMaterialInstance` (`self.Cube`) 0 "/Game/Materials/M_KillVolume.M_KillVolume" "None"))
  (set `self.Cube Material` _returnvalue))

(event `self.ReceiveTick`
  (params (DeltaSeconds :type "Float (single-precision)"))
  (bind _cube_material (`self.Cube Material`))
  (`KismetSystemLibrary.Delay` 1.0)
  (`/Engine/EditorBlueprintResources/StandardMacros.FlipFlop`
    (:`A`
      (`MaterialInstanceDynamic.SetVectorParameterValue` _cube_material "Second Base Color" (struct :`R` 1.0 :`G` 0.205923 :`A` 1.0)))
    (:`B`
      (`MaterialInstanceDynamic.SetVectorParameterValue` _cube_material "Second Base Color" (struct :`R` 1.0 :`A` 1.0)))))

(event `self.Box.OnComponentBeginOverlap`
  (params (OverlappedComponent :type "PrimitiveComponent Object Reference") (OtherActor :type "Actor Object Reference") (OtherComp :type "PrimitiveComponent Object Reference") (OtherBodyIndex :type Integer) (bFromSweep :type Boolean) (SweepResult :type "HitResult Structure (by ref)"))
  (`GameplayStatics.OpenLevel` "GameOverMap"))

(fn `UserConstructionScript`)