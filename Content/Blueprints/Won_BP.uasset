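; Won_BP is a level-exit goal actor that opens the level named by LevelToOpen when anything begins overlapping its Box, with no actor filter.
; Tick spins two static meshes on pitch and roll respectively by a fixed per-frame step, so speed depends on frame rate.
; A short Delay in Tick throttles the PointLight's changes to random colors, producing a disco-like flicker.
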(event `self.ReceiveTick`
  (params (DeltaSeconds :type "Float (single-precision)"))
  (`SceneComponent.K2_AddLocalRotation` (`self.StaticMesh1`) (`KismetMathLibrary.MakeRotator` 0.0 2.0) false false)
  (`SceneComponent.K2_AddLocalRotation` (`self.StaticMesh2`) (`KismetMathLibrary.MakeRotator` 2.0) false false)
  (`KismetSystemLibrary.Delay` 0.1)
  (`LightComponent.SetLightColor` (`self.PointLight`) (make `LinearColor` (`KismetMathLibrary.RandomFloatInRange` 0.0 1.0) (`KismetMathLibrary.RandomFloatInRange` 0.0 1.0) (`KismetMathLibrary.RandomFloatInRange` 0.0 1.0) 1.0) true))

(event `self.Box.OnComponentBeginOverlap`
  (params (OverlappedComponent :type "PrimitiveComponent Object Reference") (OtherActor :type "Actor Object Reference") (OtherComp :type "PrimitiveComponent Object Reference") (OtherBodyIndex :type Integer) (bFromSweep :type Boolean) (SweepResult :type "HitResult Structure (by ref)"))
  (`GameplayStatics.OpenLevel` (`self.Level To Open`)))

(fn `UserConstructionScript`)